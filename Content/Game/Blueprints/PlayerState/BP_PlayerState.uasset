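; BP_PlayerState is the player state that keeps health persistent through BP_GameInstance and triggers respawn on death.
; On BeginPlay it either restores saved current and max health into its health component and rebroadcasts the change, or resets health on first initialization.
; Each health change event writes both values back to the game instance.
; The death event calls Respawn on BP_ThirdPersonGameMode for player controller 0.
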(event `self.ReceiveBeginPlay`
  (bind _asbp_game_instance (cast `/Game/Game/Blueprints/BP_GameInstance` (`GameplayStatics.GetGameInstance`)))
  (bind _output_get (set `self.RefGameInstance` _asbp_game_instance))
  (if (`/Game/Game/Blueprints/BP_GameInstance.InisialisationVie_GI` _output_get)
    (`self.LoadVie`)
    (else
      (`/Game/Game/Blueprints/Components/AC_Health.ResetHealth` (`self.AC_Health`))
      (set `/Game/Game/Blueprints/BP_GameInstance.InisialisationVie_GI` true _output_get))))

(event `self.AC_Health.ChangementVie`
  (params (VieActuel :type "Float (double-precision)") (VieMaximum :type "Float (double-precision)"))
  (`self.SauvegarderVieActuel` VieActuel)
  (`self.SauvegarderVieMaximum` VieMaximum))

(event `self.AC_Health.Mourut`
  (bind _asbp_third_person_game_mode (cast `/Game/Game/Blueprints/GameModes/BP_ThirdPersonGameMode` (`GameplayStatics.GetGameMode`)))
  (`/Game/Game/Blueprints/GameModes/BP_ThirdPersonGameMode.Respawn` _asbp_third_person_game_mode (`GameplayStatics.GetPlayerController` 0)))

(fn `LoadVie`
  (bind _refgameinstance (`self.RefGameInstance`))
  (bind _ac_health (`self.AC_Health`))
  (bind _output_get (set `/Game/Game/Blueprints/Components/AC_Health.VieMaximum` (`/Game/Game/Blueprints/BP_GameInstance.VieMaximum_GI` _refgameinstance) _ac_health))
  (bind _output_get_2 (set `/Game/Game/Blueprints/Components/AC_Health.VieActuel` (`/Game/Game/Blueprints/BP_GameInstance.VieActuel_GI` _refgameinstance) _ac_health))
  (`/Game/Game/Blueprints/Components/AC_Health.ChangementVie` (`self.AC_Health`) _output_get_2 _output_get))

(fn `SauvegarderVieActuel`
  (params (NouvelleVie :type "Float (double-precision)"))
  (set `/Game/Game/Blueprints/BP_GameInstance.VieActuel_GI` NouvelleVie (`self.RefGameInstance`)))

(fn `SauvegarderVieMaximum`
  (params (NouvelleVieMaximum :type "Float (double-precision)"))
  (set `/Game/Game/Blueprints/BP_GameInstance.VieMaximum_GI` NouvelleVieMaximum (`self.RefGameInstance`)))

(fn `UserConstructionScript`)