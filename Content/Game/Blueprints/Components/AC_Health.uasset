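; Health component that tracks current and maximum health and a dead state, with events for damage, healing and reset.
; UpdateVie clamps the new value, broadcasts ChangementVie, and at zero sets Mort and broadcasts Mourut.
; Damage and healing are ignored while dead, and ResetHealth revives to maximum.
; TakeDamage passes damage minus current health, the reverse of a usual subtraction, so any hit not exceeding current health kills.
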(event `/Game/Game/Blueprints/Interfaces/BPI_Damageable.TakeDamage`
  (params (`PointDeDégât` :type "Float (double-precision)"))
  (if (not (`self.Mort`))
    (`self.UpdateVie` (- `PointDeDégât` (`self.VieActuel`)))))

(event `/Game/Game/Blueprints/Interfaces/BPI_Damageable.GainHealth`
  (params (PointDeSoin :type "Float (double-precision)"))
  (if (not (`self.Mort`))
    (`self.UpdateVie` (+ PointDeSoin (`self.VieActuel`)))))

(event `/Game/Game/Blueprints/Interfaces/BPI_Damageable.ResetHealth`
  (set `self.Mort` false)
  (`self.UpdateVie` (`self.VieMaximum`)))

(fn `UpdateVie`
  (params (ValeurVieActuel :type "Float (double-precision)"))
  (bind _viemaximum (`self.VieMaximum`))
  ; Permet de mettre à jour le système de vie
  (bind _output_get (set `self.VieActuel` (`KismetMathLibrary.FClamp` ValeurVieActuel 0.0 _viemaximum)))
  (`self.ChangementVie` _output_get _viemaximum)
  (if (<= (`self.VieActuel`) 0.0)
    (set `self.Mort` true)
    (`self.Mourut`)
    (else
      (set `self.Mort` false))))